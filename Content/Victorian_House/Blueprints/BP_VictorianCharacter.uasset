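; First-person player character for the Victorian house, handling object focus, interaction, book inspection and autofocus depth of field.
; In edit mode, short camera traces send focus messages each tick and interact messages on left click.
; Clicking also toggles book inspection, stopping movement and moving the book via a timeline, with helpers to yaw and roll it.
; A looping timer traces ahead to set camera focal distance, and BeginPlay adds the edit-mode widget.
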(event Custom|EditeModeOn
  ;[1 1 1] Interaction
  ;;[1 1 1] EditeMode
  (Variables|Default|SetEditMode%20%28on/off%29 true))

(event Custom|OutInspection
  ;[1 1 1] Inspection
  (Utilities|FlowControl|Sequence
    (:then_0
      (Utilities|FlowControl|Delay 1.0)
      (Variables|Default|SetStopMovement false)
      (Variables|Default|SetIsInspecting false))
    (:then_1
      (Variables|Default|SetSetInspectionObject 0)
      (bind _moveactor (Timeline|MoveObject Reverse)
        (:Update
          (Variables|Default|SetMoveActor _moveactor)
          (Transformation|SetActorLocationAndRotation (stale Input|MouseEvents|LeftMouseButton _asbp_book_inspection) (Math|Vector|Lerp(Vector) (Variables|Default|GetInspectionObjectLocation) (Transformation|GetWorldLocation (Variables|Default|GetInspectionLocation)) (Variables|Default|GetMoveActor)) (Math|Rotator|Lerp(Rotator) (Variables|Default|GetInspectionObject) (Transformation|GetActorRotation (stale Input|MouseEvents|LeftMouseButton _asbp_book_inspection)) (Variables|Default|GetMoveActor))))))))

(event Custom|EditeModeOff
  ;[1 1 1] Interaction
  ;;[1 1 1] EditeMode
  (Variables|Default|SetEditMode%20%28on/off%29 false))

(event Custom|DOF
  (bind _firstpersoncamera (Variables|MyCharacter|GetFirstPersonCamera))
  (bind _returnvalue (Transformation|GetWorldLocation _firstpersoncamera))
  ;[1 1 1] DOF
  (bind (_outhit _returnvalue_2) (Collision|LineTraceByChannel _returnvalue (+ (* (Math|Vector|GetForwardVector _firstpersoncamera) 1e+03) _returnvalue) "TraceTypeQuery1" false 0 "None" false))
  (if _returnvalue_2
    (Variables|Default|SetFocusDistance (Math|Vector|VectorLength (- (.Location (Collision|BreakHitResult _outhit)) (Transformation|GetWorldLocation (Variables|MyCharacter|GetFirstPersonCamera)))))
    (else
      (Variables|Default|SetFocusDistance 1e+03)))
  (Variables|/Script/Engine.CameraComponent|SetPostProcessSettings (Variables|MyCharacter|GetFirstPersonCamera) (Utilities|Struct|MakePostProcessSettings (Variables|Default|GetPowerDOF) (Variables|Default|GetFocusDistance))))

(event EventBeginPlay
  ;[1 1 1] BeginPlay
  (Utilities|FlowControl|Sequence
    (:then_0
      ;[1 1 1] Interaction
      ;;[1 1 1] EditeMode
      (bind _returnvalue (UserInterface|CreateWidget "/Game/Victorian_House/UMG/Edite_Mode_Widget.Edite_Mode_Widget_C")) ; Change widget for Edit Mode
      (UserInterface|Viewport|AddtoViewport _returnvalue 0))
    (:then_1
      ;[1 1 1] DOF
      ;;[1 1 1] Begin DOF
      (Utilities|Time|SetTimerbyFunctionName 0 "DOF" 0.1 true)
      (Variables|Default|SetPowerDOF 1.0) ; Initial value DOF on
    )))

(event EventTick
  (params (DeltaSeconds :type Float%20%28single-precision%29))
  (bind _firstpersoncamera (Variables|MyCharacter|GetFirstPersonCamera))
  (bind _returnvalue (Transformation|GetWorldLocation _firstpersoncamera))
  ;[1 1 1] Outline On
  (Development|PrintString (Utilities|String|ToString(Boolean) (Variables|Default|GetIsOnLadder)))
  (if (Variables|Default|GetEditMode%20%28on/off%29)
    (bind _returnvalue_2 (Collision|LineTraceByChannel _returnvalue (+ (* (Math|Vector|GetForwardVector _firstpersoncamera) 3e+02) _returnvalue) "TraceTypeQuery1" false 0 "None"))
    (if _returnvalue_2
      (CallFunction|OutlineBegin))))

(event Input|MouseEvents|LeftMouseButton
  (params (Key :type Key%20Structure :default "None"))
  (bind _firstpersoncamera (Variables|MyCharacter|GetFirstPersonCamera))
  (bind _returnvalue (Transformation|GetWorldLocation _firstpersoncamera))
  ;[1 1 1] Interaction
  (:Pressed
    (if (Variables|Default|GetEditMode%20%28on/off%29)
      (bind (_outhit _returnvalue_2) (Collision|LineTraceByChannel _returnvalue (+ (* (Math|Vector|GetForwardVector _firstpersoncamera) 3e+02) _returnvalue) "TraceTypeQuery1" false 0 "None"))
      (if _returnvalue_2
        (Class|BPInteractInterface|OnInteract(Message) (.HitActor (Collision|BreakHitResult _outhit)))))))

(event Input|MouseEvents|LeftMouseButton
  (params (Key :type Key%20Structure :default "None"))
  (bind _firstpersoncamera (Variables|MyCharacter|GetFirstPersonCamera))
  (bind _returnvalue (Transformation|GetWorldLocation _firstpersoncamera))
  ;[1 1 1] Inspection
  (:Pressed
    (if (Variables|Default|GetIsInspecting)
      (CallFunction|OutInspection)
      (else
        (bind _outhit (Collision|LineTraceByChannel _returnvalue (+ _returnvalue (* (Math|Vector|GetForwardVector _firstpersoncamera) 3e+02)) "TraceTypeQuery1" false 0 "None"))
        (if (.bblockinghit _outhit)
          (bind _output_get (Variables|Default|SetSetInspectionObject (.hitactor _outhit)))
          (bind _asbp_book_inspection (Utilities|Casting|CastToBP_Book_Inspection _output_get))
          (Variables|Default|SetIsInspecting true)
          (Variables|Default|SetStopMovement true)
          (Variables|Default|SetInspectionObject (Transformation|GetActorRotation _asbp_book_inspection))
          (Variables|Default|SetInspectionObjectLocation (Transformation|GetActorLocation _asbp_book_inspection))
          (bind _moveactor (Timeline|MoveObject Play)
            (:Update
              (Variables|Default|SetMoveActor _moveactor)
              (Transformation|SetActorLocationAndRotation _asbp_book_inspection (Math|Vector|Lerp(Vector) (Variables|Default|GetInspectionObjectLocation) (Transformation|GetWorldLocation (Variables|Default|GetInspectionLocation)) (Variables|Default|GetMoveActor)) (Math|Rotator|Lerp(Rotator) (Variables|Default|GetInspectionObject) (Transformation|GetActorRotation _asbp_book_inspection) (Variables|Default|GetMoveActor))))))))))

(fn ConstructionScript)

(fn OutlineBegin
  (bind _firstpersoncamera (Variables|MyCharacter|GetFirstPersonCamera))
  (bind _returnvalue (Transformation|GetWorldLocation _firstpersoncamera))
  ;[1 1 1] Outline Begin function
  (bind _outhit (Collision|LineTraceByChannel _returnvalue (+ (* (Math|Vector|GetForwardVector _firstpersoncamera) 3e+02) _returnvalue) "TraceTypeQuery1" false 0 "None"))
  (Class|BPInteractInterface|OnFocus(Message) (.HitActor (Collision|BreakHitResult _outhit))))

(fn TurnObject
  (params (Yaw :type Float%20%28double-precision%29))
  (bind _asbp_book_inspection (Utilities|Casting|CastToBP_Book_Inspection (Variables|Default|GetSetInspectionObject)))
  (Transformation|SetActorRotation _asbp_book_inspection (Math|Rotator|CombineRotators (Math|Rotator|MakeRotator 0.0 0.0 Yaw) (Transformation|GetActorRotation _asbp_book_inspection))))

(fn RollObject
  (params (Roll :type Float%20%28double-precision%29))
  (bind _asbp_book_inspection (Utilities|Casting|CastToBP_Book_Inspection (Variables|Default|GetSetInspectionObject)))
  (Transformation|SetActorRotation _asbp_book_inspection (Math|Rotator|CombineRotators (Math|Rotator|MakeRotator Roll 0.0 0.0) (Transformation|GetActorRotation _asbp_book_inspection))))