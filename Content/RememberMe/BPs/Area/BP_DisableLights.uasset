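; Trigger volume actor that toggles tagged directional lights and removes height fog as the player passes through an area.
; When the player pawn enters the Box, it hides the first ExponentialHeightFog and unhides DirectionalLights tagged "Delete" in game.
; Leaving the Box hides those lights again but does not restore the fog.
; Unconnected leftover nodes include light toggles noted for removal in the final implementation.
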(event OnComponentBeginOverlap(Box)
  (params (OverlappedComponent :type Primitive%20Component%20Object%20Reference) (OtherActor :type Actor%20Object%20Reference) (OtherComp :type Primitive%20Component%20Object%20Reference) (OtherBodyIndex :type Integer) (bFromSweep :type Boolean) (SweepResult :type Hit%20Result%20Structure%20%28by%20ref%29))
  (if (== OtherActor (Game|Player|GetPlayerPawn 0))
    (bind _outactors (Actor|GetAllActorsOfClass "/Script/Engine.ExponentialHeightFog"))
    (Rendering|SetVisibility (Variables|/Script/Engine.ExponentialHeightFog|GetComponent (Utilities|Array|Get(acopy) _outactors)) false false)
    (bind _outactors_2 (Actor|GetAllActorsOfClasswithTag "/Script/Engine.DirectionalLight" "Delete"))
    (for _array_element _outactors_2
      (Development|SetHiddeninGame (Variables|/Script/Engine.Light|GetLightComponent _array_element) false true))))

(event OnComponentEndOverlap(Box)
  (params (OverlappedComponent :type Primitive%20Component%20Object%20Reference) (OtherActor :type Actor%20Object%20Reference) (OtherComp :type Primitive%20Component%20Object%20Reference) (OtherBodyIndex :type Integer))
  (if (== OtherActor (Game|Player|GetPlayerPawn 0))
    (bind _outactors (Actor|GetAllActorsOfClasswithTag "/Script/Engine.DirectionalLight" "Delete"))
    (for _array_element _outactors
      (Development|SetHiddeninGame (Variables|/Script/Engine.Light|GetLightComponent _array_element) true true))))

(event EventBeginPlay)

(fn ConstructionScript)