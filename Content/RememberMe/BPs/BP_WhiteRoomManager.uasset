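; BP_WhiteRoomManager runs the white room sequence, playing intro subtitles on BeginPlay and staging story beats as VHSCounter rises.
; A looping timer polls the counter: from three, it plays a one-time dialogue chain, switches the middle TV on with the Mnemosyne channel, then shows narrative options.
; At five, a timeline moves the tagged RoundButton vertically into place.
; Subtitles each use a fresh widget, spaced by delays derived from their duration data.
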(event Custom|BringButtonUp
  (bind _outactors (Actor|GetAllActorsOfClasswithTag "/Game/HorrorEngine/Blueprints/UsableAssets/Controllers/RoundButton.RoundButton_C" "WhiteRoom"))
  (bind _zheight (Timeline|Timeline PlayFromStart)
    (:Update
      (Transformation|SetWorldLocation (Variables|/Script/Engine.Actor|GetRootComponent (Utilities|Array|Get(acopy) _outactors)) (Math|Vector|MakeVector (.x (Transformation|GetWorldLocation (Variables|/Script/Engine.Actor|GetRootComponent (Utilities|Array|Get(acopy) _outactors)))) (.y (Transformation|GetWorldLocation (Variables|/Script/Engine.Actor|GetRootComponent (Utilities|Array|Get(acopy) _outactors)))) _zheight) false false))))

(event Custom|CheckCounter
  (bind _doyouwho (Variables|Default|GetDoYouWho))
  (bind _subtitle3 (Variables|Default|GetSubtitle3))
  (bind _subtitle4 (Variables|Default|GetSubtitle4))
  (bind _subtitle5 (Variables|Default|GetSubtitle5))
  (bind _vhscounter (Variables|Default|GetVHSCounter))
  (if (>= _vhscounter 3)
    (if (>= _vhscounter 5)
      (Utilities|FlowControl|DoOnce false
        (:Completed
          (CallFunction|BringButtonUp)))
      (else
        (Utilities|FlowControl|DoOnce false
          (:Completed
            (bind _subtitlewidget (CallFunction|CreateSubtitleWidget))
            (Default|SubtitleText _subtitlewidget _subtitle3)
            (Utilities|FlowControl|Delay (* (.ModifyDuration+or-Sec (Utilities|Struct|BreakHE_Subtitle (Utilities|Array|Get(acopy) _subtitle3))) 1.1))
            (bind _subtitlewidget_2 (CallFunction|CreateSubtitleWidget))
            (Default|SubtitleText _subtitlewidget_2 _doyouwho)
            (Utilities|FlowControl|Delay (* (.ModifyDuration+or-Sec (Utilities|Struct|BreakHE_Subtitle (Utilities|Array|Get(acopy) _doyouwho))) 1.1))
            (bind _subtitlewidget_3 (CallFunction|CreateSubtitleWidget))
            (Default|SubtitleText _subtitlewidget_3 _subtitle4)
            (Utilities|FlowControl|Delay (* (.ModifyDuration+or-Sec (Utilities|Struct|BreakHE_Subtitle (Utilities|Array|Get(acopy) _subtitle4))) 1.1))
            (bind _subtitlewidget_4 (CallFunction|CreateSubtitleWidget))
            (Default|SubtitleText _subtitlewidget_4 _subtitle5)
            ;[0.15 0.15 0.15 0.5] Place Player in position and rotation to see all 3 screens
            (bind _outactors (Actor|GetAllActorsOfClasswithTag "/Game/HorrorEngine/Blueprints/UsableAssets/Electronics/Tv.Tv_C" "Middle"))
            (Utilities|Array|Add (Variables|/Game/HorrorEngine/Blueprints/UsableAssets/Electronics/Tv.Tv_C|GetAddChannels (Utilities|Array|Get(acopy) _outactors)) "/Game/Movies/Mnemosyne.Mnemosyne")
            (Default|Open/On (Utilities|Array|Get(acopy) _outactors) false)
            (Variables|/Game/HorrorEngine/Blueprints/UsableAssets/Electronics/Tv.Tv_C|SetOn%20/%20Off (Utilities|Array|Get(acopy) _outactors) true)
            (Utilities|FlowControl|Delay (* (.ModifyDuration+or-Sec (Utilities|Struct|BreakHE_Subtitle (Utilities|Array|Get(acopy) _subtitle5))) 1.1))
            (bind _returnvalue (UserInterface|CreateWidget "/Game/RememberMe/Widgets/WBP_NarrativeOptions.WBP_NarrativeOptions_C"))
            (UserInterface|Viewport|AddtoViewport _returnvalue 0)))))))

(event EventBeginPlay
  (bind _doyouwho (Variables|Default|GetDoYouWho))
  ;[0.15 0.15 0.15 0.5] Create new widget everytime
  (bind _subtitlewidget (CallFunction|CreateSubtitleWidget))
  (Default|SubtitleText _subtitlewidget _doyouwho)
  (Utilities|FlowControl|Delay (* (.ModifyDuration+or-Sec (Utilities|Struct|BreakHE_Subtitle (Utilities|Array|Get(acopy) _doyouwho))) 1.1))
  (bind _subtitlewidget_2 (CallFunction|CreateSubtitleWidget))
  (Default|SubtitleText _subtitlewidget_2 (Variables|Default|GetSubtitle2))
  (Utilities|Time|SetTimerbyEvent (delegate Custom|CheckCounter) 0.1 true))

(fn ConstructionScript)

(fn CreateSubtitleWidget
  (bind _returnvalue (UserInterface|CreateWidget "/Game/HorrorEngine/Blueprints/Widgets/SubtitleWB.SubtitleWB_C"))
  (UserInterface|Viewport|AddtoViewport _returnvalue 0)
  (return _returnvalue))