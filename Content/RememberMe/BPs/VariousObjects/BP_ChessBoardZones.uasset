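; Interactable chessboard puzzle where, once the player has the chess piece, interacting toggles a blended board view, locking movement and look and adding WBP_ChessTable.
; Move events step a marker within board bounds, and Check compares it to CorrectPosition.
; A match destroys board components, spawns a physics Cameroid, shows a notice, removes the last inventory item and exits.
; Focus drives a custom-depth outline cleared by retriggerable delay.
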(event Custom|MoveUp
  (if (not (> (.y (Variables|/Script/Engine.SceneComponent|GetRelativeLocation (Variables|Default|GetSelectedPosition))) 20.081309))
    (Transformation|AddRelativeLocation (Variables|Default|GetSelectedPosition) "0.000000,6.000000,0.000000" false false)))

(event Custom|MoveDown
  (if (not (< (.y (Variables|/Script/Engine.SceneComponent|GetRelativeLocation (Variables|Default|GetSelectedPosition))) -19.918691))
    (Transformation|AddRelativeLocation (Variables|Default|GetSelectedPosition) "0.000000,-6.000000,0.000000" false false)))

(event Custom|MoveLeft
  (if (not (> (.x (Variables|/Script/Engine.SceneComponent|GetRelativeLocation (Variables|Default|GetSelectedPosition))) 19.854984))
    (Transformation|AddRelativeLocation (Variables|Default|GetSelectedPosition) "6.000000,0.000000,0.000000" false false)))

(event Custom|MoveRight
  (if (not (< (.x (Variables|/Script/Engine.SceneComponent|GetRelativeLocation (Variables|Default|GetSelectedPosition))) -20.145016))
    (Transformation|AddRelativeLocation (Variables|Default|GetSelectedPosition) "-6.000000,0.000000,0.000000" false false)))

(event Custom|Check
  (if (Utilities|Operators|EqualEqual (Variables|/Script/Engine.SceneComponent|GetRelativeLocation (Variables|Default|GetSelectedPosition)) (Variables|/Script/Engine.SceneComponent|GetRelativeLocation (Variables|Default|GetCorrectPosition)) 1.0)
    (Audio|PlaySound2D "/Engine/EngineSounds/1kSineTonePing.1kSineTonePing" 1.0 1.0 0.0 0 0)
    (Components|DestroyComponent (Variables|Default|GetCorrectPosition))
    (bind _returnvalue (Game|SpawnActorfromClass "/Game/HorrorEngine/Blueprints/UsableAssets/Inventory/Cameroid.Cameroid_C" (Math|Transform|MakeTransform "-144.477705,-114.115097,198.103751" "0, 0, 0" "1.000000,1.000000,1.000000") "Undefined" "MultiplyWithRoot" 0 0))
    (Physics|SetSimulatePhysics (Variables|/Game/HorrorEngine/Blueprints/UsableAssets/Inventory/Cameroid.Cameroid_C|GetCameroidActor _returnvalue) true)
    (bind _returnvalue_2 (UserInterface|CreateWidget "/Game/HorrorEngine/Blueprints/Widgets/NoticeWB.NoticeWB_C"))
    (Variables|/Game/HorrorEngine/Blueprints/Widgets/NoticeWB.NoticeWB_C|SetFrontMessageText _returnvalue_2 "Something fell from ")
    (Variables|/Game/HorrorEngine/Blueprints/Widgets/NoticeWB.NoticeWB_C|SetItemText _returnvalue_2 "under the table")
    (Variables|/Game/HorrorEngine/Blueprints/Widgets/NoticeWB.NoticeWB_C|SetMessageText _returnvalue_2 ", looks important")
    (UserInterface|Viewport|AddtoViewport _returnvalue_2 0)
    (bind _asmaster (CallFunction|GetPlayer))
    (Utilities|Array|RemoveIndex (Variables|/Game/HorrorEngine/HorrorEngine.HorrorEngine_C|GetPlayerInventory _asmaster) (- (Utilities|Array|Length (Variables|/Game/HorrorEngine/HorrorEngine.HorrorEngine_C|GetPlayerInventory _asmaster)) 1))
    (Variables|Default|SetChessOnInventory false)
    (CallFunction|ExitChessBoard)
    (else
      (Audio|PlaySound2D "/Engine/EditorSounds/Notifications/CompileFailed.CompileFailed" 1.0 1.0 0.0 0 0))))

(event Custom|ExitChessBoard
  (bind _returnvalue (Game|GetPlayerController 0))
  ;[1 1 1] ZoomOut
  (Game|Player|SetViewTargetwithBlend _returnvalue (Game|GetPlayerCharacter 0) 1.0 "VTBlend_Linear" 0.0 true)
  (Variables|/Script/Engine.CharacterMovementComponent|SetMaxWalkSpeed (Variables|/Script/Engine.Character|GetCharacterMovement (Game|GetPlayerCharacter 0)) 1.5e+02)
  (Class|PlayerController|SetDeprecatedInputPitchScale _returnvalue -2.0)
  (Class|PlayerController|SetDeprecatedInputYawScale _returnvalue 2.0)
  (Widget|RemovefromParent (stale EventOnInteract _returnvalue_3)))

(event Input|EnhancedActionEvents|EnhancedInputActionIA_ExitFullScreen
  (params (ActionValue :type Boolean) (ElapsedSeconds :type Float%20%28double-precision%29) (TriggeredSeconds :type Float%20%28double-precision%29) (InputAction :type Input%20Action%20Object%20Reference :default "/Game/RememberMe/InputActions/IA_ExitFullScreen.IA_ExitFullScreen"))
  (CallFunction|ExitChessBoard))

(event Input|EnhancedActionEvents|EnhancedInputActionIA_SkipCutscene
  (params (ActionValue :type Boolean) (ElapsedSeconds :type Float%20%28double-precision%29) (TriggeredSeconds :type Float%20%28double-precision%29) (InputAction :type Input%20Action%20Object%20Reference :default "/Game/RememberMe/InputActions/IA_SkipCutscene.IA_SkipCutscene"))
  (CallFunction|ExitChessBoard))

(event EventBeginPlay
  (Development|SetHiddeninGame (Variables|Default|GetSelectedPosition) true true))

(event EventOnFocus
  ;[1 1 1] Outline
  (Utilities|FlowControl|Sequence
    (:then_0
      (if (Variables|Default|GetOutline%20on/off)
        (CallFunction|BeginFocus))
      (Variables|Default|SetTimeOutlineEnd 0.1)
      (Utilities|FlowControl|RetriggerableDelay (Variables|Default|GetTimeOutlineEnd))
      (CallFunction|EndFocus))
    (:then_1
      (bind _returnvalue (UserInterface|CreateWidget "/Game/RememberMe/Widgets/WBP_ChessTable.WBP_ChessTable_C" 0 0))
      (UserInterface|Viewport|AddtoViewport _returnvalue 0))))

(event EventOnInteract
  (bind _returnvalue (Game|GetPlayerController 0))
  (bind _returnvalue_2 (Game|GetPlayerController 0))
  (bind _selectedposition (Variables|Default|GetSelectedPosition))
  (if (Variables|Default|GetChessOnInventory)
    (Utilities|FlowControl|FlipFlop
      (:A
        ;[1 1 1] ZoomIn
        (Development|SetHiddeninGame _selectedposition false true)
        (Game|Player|SetViewTargetwithBlend _returnvalue self 1.0 "VTBlend_Linear" 0.0 true)
        (Variables|/Script/Engine.CharacterMovementComponent|SetMaxWalkSpeed (Variables|/Script/Engine.Character|GetCharacterMovement (Game|GetPlayerCharacter 0)) 0.0)
        (Class|PlayerController|SetDeprecatedInputPitchScale _returnvalue 0.0)
        (Class|PlayerController|SetDeprecatedInputYawScale _returnvalue 0.0)
        (bind _returnvalue_3 (UserInterface|CreateWidget "/Game/RememberMe/Widgets/WBP_ChessTable.WBP_ChessTable_C" 0 self))
        (UserInterface|Viewport|AddtoViewport _returnvalue_3 0))
      (:B
        ;[1 1 1] ZoomOut
        (Development|SetHiddeninGame _selectedposition true true)
        (Game|Player|SetViewTargetwithBlend _returnvalue_2 (Game|GetPlayerCharacter 0) 1.0 "VTBlend_Linear" 0.0 true)
        (Variables|/Script/Engine.CharacterMovementComponent|SetMaxWalkSpeed (Variables|/Script/Engine.Character|GetCharacterMovement (Game|GetPlayerCharacter 0)) 1.5e+02)
        (Class|PlayerController|SetDeprecatedInputPitchScale _returnvalue_2 -2.0)
        (Class|PlayerController|SetDeprecatedInputYawScale _returnvalue_2 2.0)
        (Widget|RemovefromParent _returnvalue_3)))
    (else
      (Development|PrintString "Find the chess piece"))))

(fn ConstructionScript)

(fn BeginFocus
  (Rendering|SetRenderCustomDepth (Variables|Default|GetChessBoard) true))

(fn EndFocus
  (Rendering|SetRenderCustomDepth (Variables|Default|GetChessBoard) false))