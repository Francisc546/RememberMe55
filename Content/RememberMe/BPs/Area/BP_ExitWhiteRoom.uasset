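; BP_ExitWhiteRoom is a trigger volume that swaps world data layers when the player leaves the white room.
; When the player pawn overlaps its Box, it activates the exit door and attic floor Data Layers and unloads the white room layer through the Data Layer Subsystem.
; It then sets a short life span so the actor destroys itself, making the transition one-shot.
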(event OnComponentBeginOverlap(Box)
  (params (OverlappedComponent :type Primitive%20Component%20Object%20Reference) (OtherActor :type Actor%20Object%20Reference) (OtherComp :type Primitive%20Component%20Object%20Reference) (OtherBodyIndex :type Integer) (bFromSweep :type Boolean) (SweepResult :type Hit%20Result%20Structure%20%28by%20ref%29))
  (if (== OtherActor (Game|Player|GetPlayerPawn 0))
    (DataLayers|SetDataLayerRuntimeState (WorldSubsystems|GetDataLayerSubsystem) (Variables|Default|GetExitDoorDataLayer) "Activated" false :!class /Script/Engine.DataLayerSubsystem)
    (DataLayers|SetDataLayerRuntimeState (WorldSubsystems|GetDataLayerSubsystem) (Variables|Default|GetWRDataLayer) "Unloaded" false :!class /Script/Engine.DataLayerSubsystem)
    (DataLayers|SetDataLayerRuntimeState (WorldSubsystems|GetDataLayerSubsystem) (Variables|Default|GetAtticFloorDataLayer) "Activated" false :!class /Script/Engine.DataLayerSubsystem)
    (Actor|SetLifeSpan 0.4)))

(fn ConstructionScript)