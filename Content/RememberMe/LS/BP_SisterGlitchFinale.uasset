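; BP_SisterGlitchFinale is a one-shot trigger actor that plays a subtitle line and then brings in the house manager.
; When the player pawn overlaps its Box, it creates a SubtitleWB widget and starts TomySubtitle from the first entry.
; After a delay slightly longer than that entry's duration, it spawns BP_HouseManager and destroys itself.
; A separate CreateVideoSubtitle helper is defined but not called within this Blueprint.
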(event OnComponentBeginOverlap(Box)
  (params (OverlappedComponent :type Primitive%20Component%20Object%20Reference) (OtherActor :type Actor%20Object%20Reference) (OtherComp :type Primitive%20Component%20Object%20Reference) (OtherBodyIndex :type Integer) (bFromSweep :type Boolean) (SweepResult :type Hit%20Result%20Structure%20%28by%20ref%29))
  (bind _tomysubtitle (Variables|Default|GetTomySubtitle))
  (if (== OtherActor (Game|Player|GetPlayerPawn 0))
    (bind _subtitlewidget (CallFunction|CreateSubtitleWidget))
    (Default|SubtitleText _subtitlewidget _tomysubtitle)
    (Utilities|FlowControl|Delay (* (.ModifyDuration+or-Sec (Utilities|Struct|BreakHE_Subtitle (Utilities|Array|Get(acopy) _tomysubtitle))) 1.05))
    (Game|SpawnActorfromClass "/Game/RememberMe/BPs/BP_HouseManager.BP_HouseManager_C" (Math|Transform|MakeTransform "0, 0, 0" "0, 0, 0" "1.000000,1.000000,1.000000") "Undefined" "MultiplyWithRoot" 0 0)
    (Actor|DestroyActor)))

(event EventBeginPlay)

(fn ConstructionScript)

(fn CreateVideoSubtitle
  (bind _returnvalue (UserInterface|CreateWidget "/Game/HorrorEngine/Blueprints/Widgets/SubtitleWB.SubtitleWB_C"))
  (UserInterface|Viewport|AddtoViewport _returnvalue 0)
  (Default|SubtitleText _returnvalue))

(fn CreateSubtitleWidget
  (bind _returnvalue (UserInterface|CreateWidget "/Game/HorrorEngine/Blueprints/Widgets/SubtitleWB.SubtitleWB_C"))
  (UserInterface|Viewport|AddtoViewport _returnvalue 0)
  (return _returnvalue))