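; Parent Blueprint for interactable actors that shows an animated input prompt and mesh outline to the player.
; When interaction is allowed, player overlap with the sphere creates a left-mouse hint widget, applies an outline overlay material and sets CanPressE.
; End overlap and HideUIInteract reverse the pop-up, then remove the widget after a short delay.
; CanReceiveTrace also toggles the hint without recreating it; the interaction itself is not handled here.
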(event OnComponentBeginOverlap(Sphere)
  (params (OverlappedComponent :type Primitive%20Component%20Object%20Reference) (OtherActor :type Actor%20Object%20Reference) (OtherComp :type Primitive%20Component%20Object%20Reference) (OtherBodyIndex :type Integer) (bFromSweep :type Boolean) (SweepResult :type Hit%20Result%20Structure%20%28by%20ref%29))
  (bind _widget (Variables|Default|GetWidget))
  (if (== OtherActor (Game|Player|GetPlayerPawn 0))
    (if (Variables|Default|GetCanInteract)
      (bind _returnvalue (UserInterface|CreateWidget "/Game/Testing/Widgets/InteractAndDirection/WBP_UIInteract.WBP_UIInteract_C" 0 "/Game/HorrorEngine/Textures/HUD/Input_MouseLeft.Input_MouseLeft"))
      (bind _output_get (Variables|Default|SetWInteract _returnvalue))
      (UserInterface|SetWidget _widget _output_get)
      (Rendering|SetVisibility _widget true false)
      (bind _winteract (Variables|Default|GetWInteract)
        (:then
          (if (not (Variables|Default|GetHintVisibility))
            (UserInterface|Animation|PlayAnimation _winteract (Variables|/Game/Testing/Widgets/InteractAndDirection/WBP_UIInteract.WBP_UIInteract_C|GetPopUp _winteract) 0.0 1 "Forward" 1.5 false)
            (Variables|Default|SetHintVisibility true)
            (CallFunction|SetMeshOverlayMaterial (Variables|Default|GetSM) "/Game/Testing/Widgets/InteractAndDirection/M_Outline.M_Outline")
            (Variables|Default|SetCanPressE true)))
        (:else)))))

(event OnComponentEndOverlap(Sphere)
  (params (OverlappedComponent :type Primitive%20Component%20Object%20Reference) (OtherActor :type Actor%20Object%20Reference) (OtherComp :type Primitive%20Component%20Object%20Reference) (OtherBodyIndex :type Integer))
  (if (== OtherActor (Game|Player|GetPlayerPawn 0))
    (if (Variables|Default|GetCanInteract)
      (bind _winteract (Variables|Default|GetWInteract)
        (:then
          (if (Variables|Default|GetHintVisibility)
            (UserInterface|Animation|PlayAnimation _winteract (Variables|/Game/Testing/Widgets/InteractAndDirection/WBP_UIInteract.WBP_UIInteract_C|GetPopUp _winteract) 0.0 1 "Reverse" 1.5 false)
            (Variables|Default|SetHintVisibility false)
            (Variables|Default|SetCanPressE false)
            (CallFunction|SetMeshOverlayMaterial (Variables|Default|GetSM))
            (Utilities|FlowControl|Delay 0.15 :!label _label)
            (Widget|RemovefromParent (Variables|Default|GetWInteract))
            (Variables|Default|SetWInteract 0)
            (Rendering|SetVisibility (Variables|Default|GetWidget) false false)))
        (:else))
      (else
        (goto _label)))))

(event Custom|HideUIInteract
  (bind _winteract (Variables|Default|GetWInteract)
    (:then
      (if (Variables|Default|GetHintVisibility)
        (UserInterface|Animation|PlayAnimation _winteract (Variables|/Game/Testing/Widgets/InteractAndDirection/WBP_UIInteract.WBP_UIInteract_C|GetPopUp _winteract) 0.0 1 "Reverse" 1.5 false)
        (Variables|Default|SetHintVisibility false)
        (Variables|Default|SetCanPressE false)
        (CallFunction|SetMeshOverlayMaterial (Variables|Default|GetSM))
        (Utilities|FlowControl|Delay 0.15)
        (Widget|RemovefromParent (Variables|Default|GetWInteract))
        (Variables|Default|SetWInteract 0)
        (Rendering|SetVisibility (Variables|Default|GetWidget) false false)))
    (:else)))

(event EventCanReceiveTrace
  (params (CanInteract :type Boolean))
  (if (Variables|Default|GetCanInteract)
    (if CanInteract
      (bind _winteract (Variables|Default|GetWInteract)
        (:then
          (if (not (Variables|Default|GetHintVisibility))
            (UserInterface|Animation|PlayAnimation _winteract (Variables|/Game/Testing/Widgets/InteractAndDirection/WBP_UIInteract.WBP_UIInteract_C|GetPopUp _winteract) 0.0 1 "Forward" 1.5 false)
            (Variables|Default|SetHintVisibility true)
            (CallFunction|SetMeshOverlayMaterial (Variables|Default|GetSM) "/Game/Testing/Widgets/InteractAndDirection/M_Outline.M_Outline")
            (Variables|Default|SetCanPressE true)))
        (:else))
      (else
        (bind _winteract_2 (Variables|Default|GetWInteract)
          (:then
            (if (Variables|Default|GetHintVisibility)
              (UserInterface|Animation|PlayAnimation _winteract_2 (Variables|/Game/Testing/Widgets/InteractAndDirection/WBP_UIInteract.WBP_UIInteract_C|GetPopUp _winteract_2) 0.0 1 "Reverse" 1.5 false)
              (Variables|Default|SetHintVisibility false)
              (CallFunction|SetMeshOverlayMaterial (Variables|Default|GetSM))
              (Variables|Default|SetCanPressE false)))
          (:else))))))

(fn ConstructionScript)

(fn SetMeshOverlayMaterial
  (params (SM :type Static%20Mesh%20Component%20Object%20Reference) (NewOverlayMaterial :type Material%20Interface%20Object%20Reference))
  (Rendering|Material|SetOverlayMaterial SM NewOverlayMaterial :!class /Script/Engine.MeshComponent))